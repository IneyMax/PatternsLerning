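; BP_ArchitecturalEngineer is the director in a Builder pattern example, driving any builder that implements BPI_ILodgingBuilder.
; The construction script validates LodgingBuilderRef and its interface through the CheckInterface macro, then caches it as PrivateLodgingBuilder.
; ConstructLodging calls the pool, restaurants, lobby and rooms message steps in fixed order.
; GetReadyLodging returns the assembled lodging message from the builder.
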(event `/Game/Patterns/Blueprints/Builder/BPI_Engineer.ConstructLodging`
  (bind _private_lodging_builder (`self.Private Lodging Builder`))
  (`|ExecutionSequence`
    (:`then_0`
      (message `/Game/Patterns/Blueprints/Builder/BPI_ILodgingBuilder.BuildSwimmingPool` _private_lodging_builder))
    (:`then_1`
      (message `/Game/Patterns/Blueprints/Builder/BPI_ILodgingBuilder.BuildRestaurants` _private_lodging_builder))
    (:`then_2`
      (message `/Game/Patterns/Blueprints/Builder/BPI_ILodgingBuilder.BuildLobbyArea` _private_lodging_builder))
    (:`then_3`
      (message `/Game/Patterns/Blueprints/Builder/BPI_ILodgingBuilder.BuildRooms` _private_lodging_builder))))

(fn `GetReadyLodging`
  (returns (ReadyLodging :type "Actor Object Reference"))
  (bind _lodging (message `/Game/Patterns/Blueprints/Builder/BPI_ILodgingBuilder.GetLodging` (`self.Private Lodging Builder`)))
  (return _lodging))

(fn `UserConstructionScript`
  (`/Engine/EditorBlueprintResources/StandardMacros.IsValid` (`self.LodgingBuilderRef`)
    (:`Is Valid`
      (`self.CheckInterface` (`self.LodgingBuilderRef`) "/Game/Patterns/Blueprints/Builder/BPI_ILodgingBuilder.BPI_ILodgingBuilder_C"
        (:`then`
          (set `self.Private Lodging Builder` (`self.LodgingBuilderRef`)))))))