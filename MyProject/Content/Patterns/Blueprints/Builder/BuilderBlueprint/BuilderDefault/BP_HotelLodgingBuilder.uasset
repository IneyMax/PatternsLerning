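; BP_HotelLodgingBuilder is a concrete builder in a Builder pattern example that assembles a luxury hotel lodging.
; On BeginPlay it spawns a BP_Lodging at its own transform and attaches it to itself.
; Each Build event sets one feature on that lodging through BPI_FloorPlan messages, guarded by a CheckInterface macro that prints when the interface is missing.
; GetLodging returns the lodging.
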(event `self.ReceiveBeginPlay`
  (`|ExecutionSequence`
    (:`then_0`
      (bind _returnvalue (`|SpawnActorFromClass` "/Game/Patterns/Blueprints/Builder/BuilderBlueprint/BP_Lodging.BP_Lodging_C" (`self.GetTransform`) "Undefined" "OverrideRootScale" null null))
      (set `self.Lodging` _returnvalue))
    (:`then_1`
      (`self.K2_AttachToActor` (`self.Lodging`) self "None" "KeepRelative" "KeepRelative" "KeepRelative" true))))

(event `/Game/Patterns/Blueprints/Builder/BuilderBlueprint/BPI_ILodgingBuilder.BuildRooms`
  (`self.CheckInterface` (`self.Lodging`) "/Game/Patterns/Blueprints/Builder/BuilderBlueprint/BPI_FloorPlan.BPI_FloorPlan_C"
    (:`then`
      (message `/Game/Patterns/Blueprints/Builder/BuilderBlueprint/BPI_FloorPlan.SetRooms` (`self.Lodging`) "5 Stars"))))

(event `/Game/Patterns/Blueprints/Builder/BuilderBlueprint/BPI_ILodgingBuilder.BuildRestaurants`
  (`self.CheckInterface` (`self.Lodging`) "/Game/Patterns/Blueprints/Builder/BuilderBlueprint/BPI_FloorPlan.BPI_FloorPlan_C"
    (:`then`
      (message `/Game/Patterns/Blueprints/Builder/BuilderBlueprint/BPI_FloorPlan.SetRestaurants` (`self.Lodging`) "Luxury"))))

(event `/Game/Patterns/Blueprints/Builder/BuilderBlueprint/BPI_ILodgingBuilder.BuildLobbyArea`
  (`self.CheckInterface` (`self.Lodging`) "/Game/Patterns/Blueprints/Builder/BuilderBlueprint/BPI_FloorPlan.BPI_FloorPlan_C"
    (:`then`
      (message `/Game/Patterns/Blueprints/Builder/BuilderBlueprint/BPI_FloorPlan.SetLobbyArea` (`self.Lodging`) "GrandHall"))))

(event `/Game/Patterns/Blueprints/Builder/BuilderBlueprint/BPI_ILodgingBuilder.BuildSwimmingPool`
  (`self.CheckInterface` (`self.Lodging`) "/Game/Patterns/Blueprints/Builder/BuilderBlueprint/BPI_FloorPlan.BPI_FloorPlan_C"
    (:`then`
      (message `/Game/Patterns/Blueprints/Builder/BuilderBlueprint/BPI_FloorPlan.SetSwimmingPool` (`self.Lodging`) "IndoorLagoon"))))

(fn `GetLodging`
  (returns (Lodging :type "Actor Object Reference"))
  (return (`self.Lodging`)))

(fn `UserConstructionScript`)