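; BP_ArchitecturalEngineerObject acts as the director in a Builder pattern example, directing the construction of a lodging.
; ConstructLodging checks that LodgingBuilderRef is valid and implements BPI_ILodgingBuilder, then sends build messages for pool, restaurants, lobby and rooms in fixed order.
; GetReadyLodging returns the finished lodging from that builder.
; Interface messages keep the construction sequence separate from how each builder makes the parts.
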(event `/Game/Patterns/Blueprints/Builder/BuilderBlueprint/BPI_Engineer.ConstructLodging`
  (bind _lodging_builderref (`self.Lodging BuilderRef`))
  (bind _lodging_builderref_2 (`self.Lodging BuilderRef`)
    (:`then`
      (if (`KismetSystemLibrary.DoesImplementInterface` _lodging_builderref_2 "/Game/Patterns/Blueprints/Builder/BuilderBlueprint/BPI_ILodgingBuilder.BPI_ILodgingBuilder_C")
        (`|ExecutionSequence`
          (:`then_0`
            (message `/Game/Patterns/Blueprints/Builder/BuilderBlueprint/BPI_ILodgingBuilder.BuildSwimmingPool` _lodging_builderref))
          (:`then_1`
            (message `/Game/Patterns/Blueprints/Builder/BuilderBlueprint/BPI_ILodgingBuilder.BuildRestaurants` _lodging_builderref))
          (:`then_2`
            (message `/Game/Patterns/Blueprints/Builder/BuilderBlueprint/BPI_ILodgingBuilder.BuildLobbyArea` _lodging_builderref))
          (:`then_3`
            (message `/Game/Patterns/Blueprints/Builder/BuilderBlueprint/BPI_ILodgingBuilder.BuildRooms` _lodging_builderref)))))
    (:`else`)))

(fn `GetReadyLodging`
  (returns (ReadyLodging :type "Actor Object Reference"))
  (bind _lodging_builderref (`self.Lodging BuilderRef`)
    (:`then`
      (bind _lodging (message `/Game/Patterns/Blueprints/Builder/BuilderBlueprint/BPI_ILodgingBuilder.GetLodging` _lodging_builderref))
      (return _lodging))
    (:`else`)))