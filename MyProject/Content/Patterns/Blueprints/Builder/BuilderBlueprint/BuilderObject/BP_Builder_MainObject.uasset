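; Client actor demonstrating the Builder design pattern with UObjects, assembling a hotel lodging on BeginPlay.
; It constructs a hotel builder object and passes it to an architectural engineer object, which acts as the director.
; The engineer constructs and returns the finished lodging, which is cast to BP_Lodging to report its characteristics, printing a failure message if the cast fails.
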(event `self.ReceiveBeginPlay`
  (bind _hotelbuilder_ (`self.SetHotelBuilder `))
  (bind _engineer (`self.SetEngineer` _hotelbuilder_))
  (message `/Game/Patterns/Blueprints/Builder/BuilderBlueprint/BPI_Engineer.ConstructLodging` _engineer)
  (bind _lodging (`self.SetLodging`))
  (bind _asbp_lodging (cast `/Game/Patterns/Blueprints/Builder/BuilderBlueprint/BP_Lodging` _lodging)
    (:`then`
      (`/Game/Patterns/Blueprints/Builder/BuilderBlueprint/BP_Lodging.LodgingCharacteristics` _asbp_lodging))
    (:`CastFailed`
      (`KismetSystemLibrary.PrintString` "FailedBuildHotel"))))

(fn `SetEngineer`
  (params (LodgingBuilderRef :type "Object Object Reference"))
  (returns (Engineer :type "/Game/Patterns/Blueprints/Builder/BuilderBlueprint/BuilderObject/BP_ArchitecturalEngineerObject Object Reference"))
  (bind _returnvalue (`|GenericCreateObject` "/Game/Patterns/Blueprints/Builder/BuilderBlueprint/BuilderObject/BP_ArchitecturalEngineerObject.BP_ArchitecturalEngineerObject_C" self LodgingBuilderRef))
  (bind _output_get (set `self.Engineer` _returnvalue))
  (return _output_get))

(fn `SetHotelBuilder `
  (returns (`HotelBuilder ` :type "/Game/Patterns/Blueprints/Builder/BuilderBlueprint/BuilderObject/BP_HotelLodgingBuilderObject Object Reference"))
  (bind _returnvalue (`|GenericCreateObject` "/Game/Patterns/Blueprints/Builder/BuilderBlueprint/BuilderObject/BP_HotelLodgingBuilderObject.BP_HotelLodgingBuilderObject_C" self))
  (bind _output_get (set `self.HotelBuilder ` _returnvalue))
  (return _output_get))

(fn `SetLodging`
  (returns (Lodging :type "Actor Object Reference"))
  (bind _readylodging (message `/Game/Patterns/Blueprints/Builder/BuilderBlueprint/BPI_Engineer.GetReadyLodging` (`self.Engineer`)))
  (bind _output_get (set `self.Lodging` _readylodging))
  (return _output_get))

(fn `UserConstructionScript`)