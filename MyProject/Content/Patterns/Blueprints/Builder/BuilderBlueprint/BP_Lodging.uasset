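; BP_Lodging is the lodging object in a Builder pattern example, holding restaurants, rooms, lobby area and swimming pool properties.
; Four setter events each store the passed value in the matching variable.
; LodgingCharacteristics prints the four stored values in sequence to show the assembled result.
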(event `/Game/Patterns/Blueprints/Builder/BuilderBlueprint/BPI_FloorPlan.SetRestaurants`
  (params (Restaurants :type String))
  (set `self.Restaurants` Restaurants))

(event `/Game/Patterns/Blueprints/Builder/BuilderBlueprint/BPI_FloorPlan.SetRooms`
  (params (Rooms :type String))
  (set `self.Rooms` Rooms))

(event `/Game/Patterns/Blueprints/Builder/BuilderBlueprint/BPI_FloorPlan.SetLobbyArea`
  (params (LobbyArea :type String))
  (set `self.Lobby Area` LobbyArea))

(event `/Game/Patterns/Blueprints/Builder/BuilderBlueprint/BPI_FloorPlan.SetSwimmingPool`
  (params (SwimmingPool :type String))
  (set `self.Swimming Pool` SwimmingPool))

(fn `LodgingCharacteristics`
  (`|ExecutionSequence`
    (:`then_0`
      (`KismetSystemLibrary.PrintString` (`self.Restaurants`) true true (struct :`G` 0.66 :`B` 1.0 :`A` 1.0) 20.0))
    (:`then_1`
      (`KismetSystemLibrary.PrintString` (`self.Rooms`) true true (struct :`G` 0.66 :`B` 1.0 :`A` 1.0) 20.0))
    (:`then_2`
      (`KismetSystemLibrary.PrintString` (`self.Lobby Area`) true true (struct :`G` 0.66 :`B` 1.0 :`A` 1.0) 20.0))
    (:`then_3`
      (`KismetSystemLibrary.PrintString` (`self.Swimming Pool`) true true (struct :`G` 0.66 :`B` 1.0 :`A` 1.0) 20.0))))

(fn `UserConstructionScript`)