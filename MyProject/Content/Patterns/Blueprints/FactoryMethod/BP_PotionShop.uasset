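; BP_PotionShop is the base creator in a Factory Method pattern example, a shop that takes potion orders.
; OrderPotion passes the requested category to ConcoctPotion, then hands the resulting potion to PreparePotion.
; ConcoctPotion is an empty factory method, leaving potion creation to child shops.
; PreparePotion runs a fixed Boil, Bubble, Brew and Bottle sequence, printing the potion's name after boiling, and returns it.
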(fn `ConcoctPotion `
  (params (PotionSKU :type String))
  (returns (Potion :type "/Game/Patterns/Blueprints/FactoryMethod/BP_Potion Object Reference"))
  (return null))

(fn `OrderPotion `
  (params (Category :type String))
  (returns (Potion :type "/Game/Patterns/Blueprints/FactoryMethod/BP_Potion Object Reference"))
  (bind _potion (`self.ConcoctPotion ` Category))
  (bind _preparedpotion (`self.PreparePotion` _potion))
  (return _preparedpotion))

(fn `PreparePotion`
  (params (Potion :type "/Game/Patterns/Blueprints/FactoryMethod/BP_Potion Object Reference"))
  (returns (PreparedPotion :type "/Game/Patterns/Blueprints/FactoryMethod/BP_Potion Object Reference"))
  (`|ExecutionSequence`
    (:`then_1`
      (`/Game/Patterns/Blueprints/FactoryMethod/BP_Potion.Boil` Potion)
      (`KismetSystemLibrary.PrintString` (`KismetStringLibrary.Concat_StrStr` "Concoct" (`/Game/Patterns/Blueprints/FactoryMethod/BP_Potion.GetPotionName` Potion)) true true (struct :`R` 0.964686 :`B` 0.637597 :`A` 1.0) 20.0))
    (:`then_2`
      (`/Game/Patterns/Blueprints/FactoryMethod/BP_Potion.Bubble` Potion))
    (:`then_3`
      (`/Game/Patterns/Blueprints/FactoryMethod/BP_Potion.Brew` Potion))
    (:`then_4`
      (`/Game/Patterns/Blueprints/FactoryMethod/BP_Potion.Bottle` Potion))
    (:`then_5`
      (return Potion))))

(fn `UserConstructionScript`)